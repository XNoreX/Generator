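; BP_Module is a tile actor for procedural road-and-house generation, with directional X/Y sockets for neighboring tiles.
; SpawnRoads picks shuffled, compatible road modules inside the Generator's box where a line trace is clear, reserves the child's socket, reports to the Generator, then recurses through spawned tiles.
; SpawnHouse randomly places random houses on allowed sockets.
; The construction script box-traces and destroys overlapping tiles, removing them from the Generator's house list.
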(event `ReservedSocket`
  (params (Socket :type "/Generator/Generator/E_Sockets Enum" :default "NewEnumerator0"))
  (switch `/Generator/Generator/E_Sockets` Socket
    (:`NewEnumerator0`
      (`KismetArrayLibrary.Array_RemoveItem` (`self.AllowedRoadsSockets`) "NewEnumerator1"))
    (:`NewEnumerator1`
      (`KismetArrayLibrary.Array_RemoveItem` (`self.AllowedRoadsSockets`) "NewEnumerator0"))
    (:`NewEnumerator2`
      (`KismetArrayLibrary.Array_RemoveItem` (`self.AllowedRoadsSockets`) "NewEnumerator3"))
    (:`NewEnumerator3`
      (`KismetArrayLibrary.Array_RemoveItem` (`self.AllowedRoadsSockets`) "NewEnumerator2"))))

(fn `SpawnHouse`
  (params (Generator :type "/Generator/Generator/BP_Generator Object Reference") (HouseModules :type "Array of /Game/Generator/BP_Module Class Reference"))
  (locals (L_Generator :type "/Generator/Generator/BP_Generator Object Reference"))
  ;[1 1 1] We get available sockets for spawning buildings and randomly set the possibility of creating a building so that not every road has a tile of a building next door
  (set `local.L_Generator` Generator)
  (bind _output_get (set `self.HouseModules` HouseModules))
  (if (`KismetMathLibrary.RandomBool`)
    (for _array_element (`self.AllowedHouseSockets`)
      (bind _returnvalue (select `/Generator/Generator/E_Sockets` _array_element :`NewEnumerator0` (`self.X`) :`NewEnumerator1` (`self.-X`) :`NewEnumerator2` (`self.Y`) :`NewEnumerator3` (`self.-Y`)))
      (bind _returnvalue_2 (`SceneComponent.GetForwardVector` _returnvalue))
      ;[1 1 1] Creating a random building from an array of available house tiles
      (bind _returnvalue_3 (`|SpawnActorFromClass` :`Class` (`KismetArrayLibrary.Array_Random` _output_get) :`SpawnTransform` (`KismetMathLibrary.MakeTransform` (+ (`SceneComponent.K2_GetComponentLocation` _returnvalue) (* _returnvalue_2 100.0)) (`KismetMathLibrary.Conv_VectorToRotator` _returnvalue_2)) :`CollisionHandlingOverride` "AdjustIfPossibleButDontSpawnIfColliding" :`TransformScaleMethod` "OverrideRootScale" :`Generator` null :`Instigator` null))
      (`KismetArrayLibrary.Array_Add` (`/Generator/Generator/BP_Generator.SpawnedHouses` (`local.L_Generator`)) _returnvalue_3))))

(fn `SpawnRoads`
  (locals (L_SocketLocation :type "Vector Structure" :default (0.0 0.0 0.0)) (L_End :type "Vector Structure") (L_Foravard :type "Vector Structure" :default (0.0 0.0 0.0)) (L_Socket :type "/Generator/Generator/E_Sockets Enum") (L_RelativeRotation :type "Rotator Structure" :default (struct)))
  (bind _returnvalue (select `/Generator/Generator/E_Sockets` (`local.L_Socket`) :`NewEnumerator0` (`self.X`) :`NewEnumerator1` (`self.-X`) :`NewEnumerator2` (`self.Y`) :`NewEnumerator3` (`self.-Y`)))
  (bind _returnvalue_2 (`SceneComponent.K2_GetComponentLocation` _returnvalue))
  (bind (_origin _boxextent) (`KismetSystemLibrary.GetComponentBounds` (`/Generator/Generator/BP_Generator.Box` (`self.Generator`))))
  (bind _returnvalue_3 (`SceneComponent.GetForwardVector` _returnvalue))
  (for _array_element (`self.AllowedRoadsSockets`)
    (set `local.L_Socket` _array_element)
    (`KismetArrayLibrary.Array_Shuffle` (`self.RoadModules`))
    ;[1 1 1] We get the correspondence with the socket
    (for _array_element_2 (`self.RoadModules`)
      (if (not (== (`KismetArrayLibrary.Array_Find` (`self.AllowedRoadModuleType`) (defaults `Object` _array_element_2)) -1))
        ;[1 1 1] If the socket is found, then we get it from the list and its parameters
        (set `local.L_SocketLocation` _returnvalue_2)
        (set `local.L_End` (+ _returnvalue_2 (* _returnvalue_3 100.0)))
        (set `local.L_Foravard` _returnvalue_3)
        (set `local.L_RelativeRotation` (`SceneComponent.RelativeRotation` _returnvalue))
        ;[1 1 1] Checking for the location of the spawn point in a collision
        (if (`KismetMathLibrary.IsPointInBox` (`local.L_SocketLocation`) _origin _boxextent)
          ;[1 1 1] Checking for neighboring sockets in the spawn direction
          (bind _outhit (`KismetSystemLibrary.LineTraceSingleForObjects` (`local.L_SocketLocation`) (`local.L_End`) (`|MakeArray` "ObjectTypeQuery2" :!type "EObjectTypeQuery Enum") false (`|MakeArray` self :!type "Actor Object Reference") "None" true (struct :`R` 1.0 :`A` 1.0) (struct :`R` 0.176475 :`B` 1.0 :`A` 1.0)))
          (`/Engine/EditorBlueprintResources/StandardMacros.IsValid` (`.HitActor` (`GameplayStatics.BreakHitResult` _outhit))
            (:`Is Valid`
              (break))
            (:`Is Not Valid`
              ;[1 1 1] Tile spawn and socket booking are reversed
              (bind _returnvalue_4 (`|SpawnActorFromClass` _array_element_2 (`KismetMathLibrary.MakeTransform` (+ (`local.L_SocketLocation`) (* (`local.L_Foravard`) 100.0)) (`local.L_RelativeRotation`)) "AlwaysSpawn" "OverrideRootScale" null (`self.RoadModules`) (`self.Generator`) null))
              (`self.ReservedSocket` _returnvalue_4 (`local.L_Socket`))
              (`KismetArrayLibrary.Array_Add` (`self.SpawnedModule`) _returnvalue_4)
              (break)))))))
  ;[1 1 1] Spawn New Tile
  (`/Generator/Generator/BP_Generator.UpdateIterationInfo` (`self.Generator`) self)
  (for _array_element_3 (`self.SpawnedModule`)
    (`self.SpawnRoads` _array_element_3)))

(fn `UserConstructionScript`
  (bind (_origin _boxextent) (`KismetSystemLibrary.GetComponentBounds` (`self.StaticMesh`)))
  (bind (_origin_2 _boxextent_2) (`KismetSystemLibrary.GetComponentBounds` (`self.StaticMesh`)))
  ;[1 1 1] Logic for destroy actor house inside actor house
  (bind _outhit (`KismetSystemLibrary.BoxTraceSingleForObjects` (`KismetMathLibrary.MakeVector` (.x _origin) (.y _origin) (.z _boxextent)) _origin_2 (/ _boxextent_2 1.5) (`self.K2_GetActorRotation`) (`|MakeArray` "ObjectTypeQuery2" :!type "EObjectTypeQuery Enum") false (`|MakeArray` (`self.Generator`) :!type "Actor Object Reference")))
  (`/Engine/EditorBlueprintResources/StandardMacros.IsValid` (`.HitActor` (`GameplayStatics.BreakHitResult` _outhit))
    (:`Is Valid`
      (`KismetArrayLibrary.Array_RemoveItem` (`/Generator/Generator/BP_Generator.SpawnedHouses` (`self.Generator`)) self)
      (`self.K2_DestroyActor`))))