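; Procedural level generator actor that spawns road tiles and houses within a box area sized from AreaSize.
; On BeginPlay or GenerateRoads it destroys old roads, spawns a random first module at the box's -X edge and calls its SpawnRoads.
; Modules receive a generator reference, and UpdateIterationInfo records them in SpawnedRoads.
; GenerateHouse has each road spawn houses, and separate events clear roads, houses or all modules.
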(event `UpdateIterationInfo`
  (params (Module :type "/Generator/Generator/BP_Module Object Reference (by ref)"))
  (`KismetArrayLibrary.Array_Add` (`self.SpawnedRoads`) Module))

(event `self.ReceiveBeginPlay`
  (bind (_origin _boxextent) (`KismetSystemLibrary.GetComponentBounds` (`self.Box`)))
  ;[1 1 1] We delete the previous generation of roads, select a random first tile and create it from the edge of the collision
  (for _array_element (`self.SpawnedRoads`) :!label _label
    (`self.K2_DestroyActor` _array_element))
  (bind _returnvalue (`|SpawnActorFromClass` (`KismetArrayLibrary.Array_Random` (`self.RoadModules`)) (`KismetMathLibrary.MakeTransform` (`KismetMathLibrary.MakeVector` (- (.x _origin) (.x _boxextent)))) "Undefined" "OverrideRootScale" null (`self.RoadModules`) self null))
  (`/Generator/Generator/BP_Module.SpawnRoads` _returnvalue))

(event `GenerateRoads`
  ;[1 1 1] We delete the previous generation of roads, select a random first tile and create it from the edge of the collision
  (goto _label))

(event `ClearRoads`
  (bind _spawnedroads (`self.SpawnedRoads`))
  ;[1 1 1] Clear Roads
  (for (_array_element _array_index) _spawnedroads
    (`self.K2_DestroyActor` _array_element)
    (`KismetArrayLibrary.Array_Remove` _spawnedroads _array_index)))

(event `ClearHouse`
  (bind _spawnedhouses (`self.SpawnedHouses`))
  ;[1 1 1] ClearHouse
  (for (_array_element _array_index) _spawnedhouses
    (`self.K2_DestroyActor` _array_element)
    (`KismetArrayLibrary.Array_Remove` _spawnedhouses _array_index)))

(event `ClearAll`
  ;[1 1 1] Clear All Tiles
  (bind _outactors (`GameplayStatics.GetAllActorsOfClass` "/Generator/Generator/BP_Module.BP_Module_C"))
  (for _array_element _outactors
    (`self.K2_DestroyActor` _array_element))
  (`KismetArrayLibrary.Array_Clear` (`self.SpawnedRoads`))
  (`KismetArrayLibrary.Array_Clear` (`self.SpawnedHouses`)))

(event `GenerateHouse`
  ;[1 1 1] We get all the road tiles and in each of them we call the logic of building tiles spawn
  (for _array_element (`self.SpawnedHouses`)
    (`self.K2_DestroyActor` _array_element))
  (for _array_element_2 (`self.SpawnedRoads`)
    (`/Generator/Generator/BP_Module.SpawnHouse` _array_element_2 self (`self.HouseModules`))))

(fn `UserConstructionScript`
  (bind (_returnvalue_x _returnvalue_y) (`KismetMathLibrary.BreakVector` (* (`self.AreaSize`) (10.0 10.0 0.0))))
  ;[1 1 1] Set Collision Size
  (`BoxComponent.SetBoxExtent` (`self.Box`) (`KismetMathLibrary.MakeVector` _returnvalue_x _returnvalue_y 500.0) true))